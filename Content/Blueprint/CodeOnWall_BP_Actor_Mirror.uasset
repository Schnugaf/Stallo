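; Mirror actor, apparently for a code-on-wall interaction, that stays hidden until revealed and can be turned in small steps.
; BeginPlay and ExitInteract share one path that hides the actor and adds a fixed rotation offset to its root.
; MirrorReflecton unhides it, and each Rotate call adds a small yaw step while world yaw is negative.
; Rotate writes the combined world rotation back as relative rotation.
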(event `self.ReceiveBeginPlay`
  (`self.SetActorHiddenInGame` true :!label _label)
  (`SceneComponent.K2_AddRelativeRotation` (`self.DefaultSceneRoot`) (struct :`Yaw` -7.0) false false))

(event `/Game/Blueprint/Interaction_BP_Root_NULL.Exit Interact`
  (goto _label))

(event `/Game/Blueprint/Interaction_BP_Root_NULL.MirrorReflecton`
  (`self.SetActorHiddenInGame` false))

(event `/Game/Blueprint/Interaction_BP_Root_NULL.Rotate`
  (bind _defaultsceneroot (`self.DefaultSceneRoot`))
  (bind (_returnvalue_roll _returnvalue_pitch _returnvalue_yaw) (`KismetMathLibrary.BreakRotator` (`SceneComponent.K2_GetComponentRotation` _defaultsceneroot)))
  (if (< _returnvalue_yaw 0.0)
    (`SceneComponent.K2_SetRelativeRotation` _defaultsceneroot (`KismetMathLibrary.ComposeRotators` (`KismetMathLibrary.MakeRotator` 0.0 0.0 1.4) (`SceneComponent.K2_GetComponentRotation` _defaultsceneroot)) false false)))

(fn `UserConstructionScript`)