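; Interactable cabinet door that swings open and closed on alternate Interact calls.
; Interact flips the Open flag and posts Wwise events, naming Cabinets only when opening.
; Tick runs OpenTimer up or down over about a second to lerp the mesh yaw between StartRot and EndRot.
; StartRot, roll and pitch come from the mesh's RelativeLocation components rather than its rotation.
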(event `/Game/Interaction_BP_Root_NULL.Interact`
  (bind _ak (`self.Ak`))
  ;[1 1 1] Interact
  (`/Engine/EditorBlueprintResources/StandardMacros.FlipFlop`
    (:`A`
      (set `self.Open` true)
      (`AkComponent.PostAkEvent` _ak "/Game/WwiseSFX/Events/GeneralHouse/Cabinets.Cabinets" ""))
    (:`B`
      (set `self.Open` false)
      (`AkComponent.PostAkEvent` _ak null ""))))

(event `self.ReceiveTick`
  (params (DeltaSeconds :type "Float (single-precision)"))
  (bind _staticmesh (`self.StaticMesh`))
  (bind (_relativelocation_x _relativelocation_y _relativelocation_z) (`KismetMathLibrary.BreakVector` (`SceneComponent.RelativeLocation` _staticmesh)))
  ;[1 1 1] Tick lerp of door
  (if (`self.Open`)
    (if (not (> (stale _output_get) 1.0))
      (bind _output_get (set `self.OpenTimer` (+ (stale _output_get) DeltaSeconds)))
      (`SceneComponent.K2_SetRelativeRotation` _staticmesh (`KismetMathLibrary.MakeRotator` _relativelocation_x _relativelocation_y (`KismetMathLibrary.Lerp` (`self.StartRot`) (`self.EndRot`) (`self.OpenTimer`))) false false :!label _label))
    (elif (not (< (stale _output_get_2) 0.001))
      (bind _output_get_2 (set `self.OpenTimer` (- (stale _output_get_2) DeltaSeconds)))
      (goto _label))))

(event `self.ReceiveBeginPlay`
  (bind (_relativelocation_x _relativelocation_y _relativelocation_z) (`KismetMathLibrary.BreakVector` (`SceneComponent.RelativeLocation` (`self.StaticMesh`))))
  ;[1 1 1] Tick lerp of door
  (set `self.StartRot` _relativelocation_z))

(fn `UserConstructionScript`)