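; An openable door actor that swings open or closed each time it receives an Interact event.
; Interact toggles IsOpen and plays the DoorSwing timeline forward or in reverse.
; The timeline's OpenAngle yaw is combined with the rotation saved at BeginPlay, so the swing is relative to the door's starting orientation.
; A Sound Timing event track on the timeline plays the Collapse01 sound at the door's location.
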(event `self.ReceiveBeginPlay`
  (set `self.Initial Rotation` (`self.K2_GetActorRotation`)))

(event `/Game/Blueprint/Interaction_BP_Root_NULL.Interact`
  (if (`self.isOpen`)
    (set `self.isOpen` false)
    (bind (_direction _open_angle) (`Timeline|Door Swing` :!via `Reverse` :!label _label)
      (:`Update`
        (`self.K2_SetActorRotation` (`KismetMathLibrary.ComposeRotators` (`self.Initial Rotation`) (`KismetMathLibrary.MakeRotator` 0.0 0.0 _open_angle))))
      (:`Sound Timing`
        (`GameplayStatics.PlaySoundAtLocation` "/Game/StarterContent/Audio/Collapse01.Collapse01" (`self.K2_GetActorLocation`))))
    (else
      (set `self.isOpen` true)
      (goto _label))))

(fn `UserConstructionScript`)