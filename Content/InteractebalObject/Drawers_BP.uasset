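; Interactable drawer actor that slides open and closed along its local Y axis with Wwise audio.
; Interact alternates between open and closed through a FlipFlop, setting the Drawer Wwise state before posting the sound event.
; Tick counts a timer up or down over about one second, lerping the mesh between the position saved at BeginPlay and Endpos, so reversals continue from mid-slide.
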(event `/Game/Interaction_BP_Root_NULL.Interact`
  (bind _ak (`self.Ak`))
  (`/Engine/EditorBlueprintResources/StandardMacros.FlipFlop`
    (:`A`
      (set `self.Open` true)
      (`AkGameplayStatics.SetState` "Drawer" "Open")
      (`AkComponent.PostAkEvent` _ak "/Game/WwiseSFX/Events/GeneralHouse/Drawers.Drawers" ""))
    (:`B`
      (set `self.Open` false)
      (`AkGameplayStatics.SetState` "Drawer" "Close")
      (`AkComponent.PostAkEvent` _ak "/Game/WwiseSFX/Events/GeneralHouse/Drawers.Drawers" ""))))

(event `self.ReceiveTick`
  (params (DeltaSeconds :type "Float (single-precision)"))
  (bind _staticmesh (`self.StaticMesh`))
  (bind (_relativelocation_x _relativelocation_y _relativelocation_z) (`KismetMathLibrary.BreakVector` (`SceneComponent.RelativeLocation` _staticmesh)))
  (if (`self.Open`)
    (if (not (> (stale _output_get) 1.0))
      (bind _output_get (set `self.OpenTimer` (+ (stale _output_get) DeltaSeconds)))
      (`SceneComponent.K2_SetRelativeLocation` _staticmesh (`KismetMathLibrary.MakeVector` _relativelocation_x (`KismetMathLibrary.Lerp` (`self.StartPos`) (`self.Endpos`) (`self.OpenTimer`)) _relativelocation_z) false false :!label _label))
    (elif (not (< (stale _output_get_2) 0.0))
      (bind _output_get_2 (set `self.OpenTimer` (- (stale _output_get_2) DeltaSeconds)))
      (goto _label))))

(event `self.ReceiveBeginPlay`
  (bind (_relativelocation_x _relativelocation_y _relativelocation_z) (`KismetMathLibrary.BreakVector` (`SceneComponent.RelativeLocation` (`self.StaticMesh`))))
  (set `self.StartPos` _relativelocation_y))

(fn `UserConstructionScript`)