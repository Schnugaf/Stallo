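; Door actor that toggles open and closed each time its Interact event is called.
; BeginPlay stores the initial rotation, and Interact flips an IsOpen flag to play or reverse a timeline.
; The timeline's OpenAngle track is applied as a yaw offset combined with that initial rotation, swinging the whole actor.
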(event `self.ReceiveBeginPlay`
  (set `self.Initial Rotation` (`self.K2_GetActorRotation`))
  (set `self.isOpen` false))

(event `/Game/Blueprint/Interaction_BP_Root_NULL.Interact`
  (if (`self.isOpen`)
    (set `self.isOpen` false)
    (bind (_direction _open_angle) (`Timeline|Timeline_0` :!via `Reverse` :!label _label)
      (:`Update`
        (`self.K2_SetActorRotation` (`KismetMathLibrary.ComposeRotators` (`self.Initial Rotation`) (`KismetMathLibrary.MakeRotator` 0.0 0.0 _open_angle)))))
    (else
      (set `self.isOpen` true)
      (goto _label))))

(fn `UserConstructionScript`)