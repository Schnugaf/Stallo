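; Quest-driven AI spawner that responds to the QuestStone1 event.
; It spawns a ThirdPersonCharacter running the MoveTowards behavior tree, taking location and rotation from arrays indexed by EventNumber.
; It then calls QuestStone1Message on the first ThirdPersonCharacter and first NPCAI_BP found in the world.
; Branches for three further spawn indices share this chain but have no triggering events, so only the first index runs.
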(event `/Game/Interaction_BP_Root_NULL.QuestStone1`
  (bind _eventnumber (`self.EventNumber`))
  (set `self.EventNumber` 0)
  (`AIBlueprintHelperLibrary.SpawnAIFromClass` "/Game/AI/ThirdPersonCPP/Blueprints/ThirdPersonCharacter.ThirdPersonCharacter_C" "/Game/AI/MoveTowards.MoveTowards" (`KismetArrayLibrary.Array_Get` (`self.SpawnLocations`) _eventnumber) (`KismetArrayLibrary.Array_Get` (`self.SpawnRotations`) _eventnumber))
  (bind _outactors (`GameplayStatics.GetAllActorsOfClass` "/Game/AI/ThirdPersonCPP/Blueprints/ThirdPersonCharacter.ThirdPersonCharacter_C"))
  (message `/Game/Interaction_BP_Root_NULL.QuestStone1` (`KismetArrayLibrary.Array_Get` _outactors))
  (bind _outactors_2 (`GameplayStatics.GetAllActorsOfClass` "/Game/AI/NPCAI_BP.NPCAI_BP_C"))
  (message `/Game/Interaction_BP_Root_NULL.QuestStone1` (`KismetArrayLibrary.Array_Get` _outactors_2)))

(fn `UserConstructionScript`)