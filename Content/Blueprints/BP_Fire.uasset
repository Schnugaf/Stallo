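; BP_Fire is an interactable fire actor with a particle effect, whose interaction works only in the Tutorial level.
; BeginPlay checks the level name to set AllowedToFire, which gates Interact setting the StartCin flag.
; Tick watches a separate Fire flag, not set in this graph, and activates the particle system through a DoOnce.
; Logic to switch the particles off exists but is unconnected.
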(event `self.ReceiveBeginPlay`
  (bind _returnvalue (`GameplayStatics.GetCurrentLevelName` true))
  (if (`KismetStringLibrary.EqualEqual_StrStr` _returnvalue "Tutorial")
    (set `self.AllowedToFire` true)
    (else
      (set `self.AllowedToFire` false))))

(event `self.ReceiveTick`
  (params (DeltaSeconds :type "Float (single-precision)"))
  (if (`self.Fire`)
    (`/Engine/EditorBlueprintResources/StandardMacros.DoOnce` false
      (:`Completed`
        (`ActorComponent.SetActive` (`self.ParticleSystem`) true true)))))

(event `/Game/Interaction_BP_Root_NULL.Interact`
  (if (`self.AllowedToFire`)
    (set `self.StartCin` true)))

(fn `UserConstructionScript`)