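; CodeOnWall is an actor, apparently a hidden code on a wall, that starts invisible and is revealed by a mirror reflection event.
; BeginPlay hides the actor, and the MirrorReflecton event shows it again.
; Each Rotate call adds one degree of yaw to the root while its world yaw is negative, writing the combined world rotation back as relative rotation.
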(event `self.ReceiveBeginPlay`
  (`self.SetActorHiddenInGame` true))

(event `/Game/Blueprint/Interationsjon_Blueprint.MirrorReflecton`
  (`self.SetActorHiddenInGame` false))

(event `/Game/Blueprint/Interationsjon_Blueprint.Rotate`
  (bind _defaultsceneroot (`self.DefaultSceneRoot`))
  (bind (_returnvalue_roll _returnvalue_pitch _returnvalue_yaw) (`KismetMathLibrary.BreakRotator` (`SceneComponent.K2_GetComponentRotation` _defaultsceneroot)))
  (if (< _returnvalue_yaw 0.0)
    (`SceneComponent.K2_SetRelativeRotation` _defaultsceneroot (`KismetMathLibrary.ComposeRotators` (`KismetMathLibrary.MakeRotator` 0.0 0.0 1.0) (`SceneComponent.K2_GetComponentRotation` _defaultsceneroot)) false false)))

(fn `UserConstructionScript`)