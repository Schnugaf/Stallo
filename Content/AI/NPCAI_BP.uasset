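; AI controller for an NPC that patrols, chases sensed targets and reacts to scripted scare and quest events.
; On BeginPlay it sets up the PatrollData blackboard and runs its behavior tree, steering it through blackboard keys.
; AI perception sets or clears EnemyKey for actors not tagged Enemy.
; QuestStone1 and MirrorScare force the player as EnemyKey, BathRoomScare sets WayPoint to the first TargetPoint found, and WaitingintheCourner is empty.
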(event `/Game/Interaction_BP_Root_NULL.BathRoomScare`
  (bind _outactors (`GameplayStatics.GetAllActorsOfClass` "/Script/Engine.TargetPoint"))
  (`BlackboardComponent.SetValueAsObject` (`self.BlackBoard Comp`) (`self.WayPoint`) (`KismetArrayLibrary.Array_Get` _outactors)))

(event `/Game/Interaction_BP_Root_NULL.WaitingInTheCourner`)

(event `/Game/Interaction_BP_Root_NULL.QuestStone1`
  (`BlackboardComponent.SetValueAsObject` (`self.BlackBoard Comp`) (`self.EnemyKey`) (`GameplayStatics.GetPlayerCharacter` 0) :!label _label))

(event `/Game/Interaction_BP_Root_NULL.MirrorScare`
  (goto _label))

(event `self.ReceiveBeginPlay`
  (bind _blackboardcomponent (`self.UseBlackboard` "/Game/AI/PatrollData.PatrollData"))
  (`self.RunBehaviorTree` "/Game/AI/Behavior.Behavior")
  (set `self.BlackBoard Comp` _blackboardcomponent))

(event `self.AIPerception.OnTargetPerceptionUpdated`
  (params (Actor :type "Actor Object Reference") (Stimulus :type "AIStimulus Structure"))
  (bind _enemykey (`self.EnemyKey`))
  (bind _blackboard_comp (`self.BlackBoard Comp`))
  ;[1 1 1] Skal få AI til å se på spilleren
  (if (`self.ActorHasTag` Actor "Enemy")
    _
    (elif (`.bSuccessfullySensed` (break `AIStimulus` Stimulus))
      (`BlackboardComponent.SetValueAsObject` _blackboard_comp _enemykey Actor)
      (else
        (`BlackboardComponent.ClearValue` _blackboard_comp _enemykey)))))

(fn `UserConstructionScript`)