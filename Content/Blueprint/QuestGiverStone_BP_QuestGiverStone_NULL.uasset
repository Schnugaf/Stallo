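; Quest stone actor with three selectable, rotatable cogwheels (TannHjul), viewed through a camera while the player interacts.
; Interact blends the player's view to the Camera's owner and sets IsInn; ExitInteract blends back to the player character and clears it.
; While IsInn is set, ChangeTarget cycles the selected wheel and Rotate adds a fixed yaw step to its world rotation, applying the result as relative rotation.
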(event `/Game/Blueprint/Interaction_BP_Root_NULL.Exit Interact`
  (`PlayerController.SetViewTargetWithBlend` (`GameplayStatics.GetPlayerController` 0) (`GameplayStatics.GetPlayerCharacter` 0) 1.0 "VTBlend_Linear" 0.0 true)
  (set `self.IsInn` false))

(event `/Game/Blueprint/Interaction_BP_Root_NULL.Interact`
  ;[1 1 1] Quest Stone 1 Camera Controll
  (`PlayerController.SetViewTargetWithBlend` (`GameplayStatics.GetPlayerController` 0) (`ActorComponent.GetOwner` (`self.Camera`)) 1.0 "VTBlend_Linear" 0.0 true)
  (set `self.IsInn` true))

(event `/Game/Blueprint/Interaction_BP_Root_NULL.ChangeTarget`
  (bind _tannhullselected (`self.TannHullSelected`))
  (if (`self.IsInn`)
    (if (> _tannhullselected 1)
      (set `self.TannHullSelected` 0)
      (else
        (set `self.TannHullSelected` (+ _tannhullselected 1))))))

(event `/Game/Blueprint/Interaction_BP_Root_NULL.Rotate`
  (bind _item (`KismetArrayLibrary.Array_Get` (`|MakeArray` (`self.TannHjull1`) (`self.TannHjull2`) (`self.TannHjull3`)) (`self.TannHullSelected`)))
  (if (`self.IsInn`)
    (`SceneComponent.K2_SetRelativeRotation` _item (`KismetMathLibrary.ComposeRotators` (`KismetMathLibrary.MakeRotator` 0.0 0.0 20.0) (`SceneComponent.K2_GetComponentRotation` _item)) false false)))

(fn `UserConstructionScript`)