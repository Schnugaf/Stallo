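; BP_LightParent is a light source Blueprint, named as a parent class, with optional candle flicker and an interactable on/off toggle.
; When IsCandle is set, Tick sets the point light's intensity and relative location from two math functions.
; Those functions hold interpolation toward clamped random intensity and small XY jitter around the BeginPlay location, though both expressions appear unconnected.
; Interact toggles the light's active state when IsInteractable is set.
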(event `self.ReceiveBeginPlay`
  (set `self.DefaultLocation` (`SceneComponent.RelativeLocation` (`self.PointLight`))))

(event `self.ReceiveTick`
  (params (DeltaSeconds :type "Float (single-precision)"))
  (if (`self.bIsCandle`)
    (`LightComponent.SetIntensity` (`self.PointLight`) (`self.DoAwesomeMath`))
    (`SceneComponent.K2_SetRelativeLocation` (`self.PointLight`) (`self.DoRadicalMath`) false false)))

(event `/Game/Interaction_BP_Root_NULL.Interact`
  (if (`self.bIsInteractable`)
    (if (`ActorComponent.IsActive` (`self.PointLight`))
      (`ActorComponent.SetActive` (`self.PointLight`) false false)
      (else
        (`ActorComponent.SetActive` (`self.PointLight`) true false)))))

(fn `UserConstructionScript`)