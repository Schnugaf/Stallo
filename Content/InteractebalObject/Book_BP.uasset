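; Interactable book Blueprint that the player opens to view pages through its own camera.
; Interact and ExitInteract swap open and closed meshes, toggle the spotlight, blend the view between book and player, and set a Wwise state before posting the sound event.
; ChangeTarget cycles through two page components with wraparound, showing only the children of the current page.
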(event `/Game/Interaction_BP_Root_NULL.Interact`
  (`AkGameplayStatics.SetState` "Book" "Open")
  (`AkComponent.PostAkEvent` (`self.Ak`) "/Game/WwiseSFX/Events/GeneralHouse/Book.Book" "")
  (`LightComponent.SetIntensity` (`self.SpotLight`) 5000.0)
  (`SceneComponent.SetVisibility` (`self.OpenBook`) true false)
  (`SceneComponent.SetVisibility` (`self.ClosedBook`) false false)
  (`PlayerController.SetViewTargetWithBlend` (`GameplayStatics.GetPlayerController` 0) (`ActorComponent.GetOwner` (`self.Camera`)) 1.0 "VTBlend_Linear" 0.0 true)
  (`SceneComponent.SetVisibility` (`SceneComponent.GetChildrenComponents` (`KismetArrayLibrary.Array_Get` (`|MakeArray` (`self.StaticMesh`) (`self.StaticMesh1`)) (`self.Page`)) false) true false))

(event `/Game/Interaction_BP_Root_NULL.ChangeTarget`
  (bind _page (`self.Page`))
  (bind _array (`|MakeArray` (`self.StaticMesh`) (`self.StaticMesh1`)))
  (bind _children (`SceneComponent.GetChildrenComponents` (`KismetArrayLibrary.Array_Get` _array _page) false))
  (`SceneComponent.SetVisibility` _children false false)
  (bind _output_get (set `self.Page` (+ (stale _output_get) 1)))
  (if (> _page (`KismetArrayLibrary.Array_LastIndex` _array))
    (set `self.Page` 0))
  (`SceneComponent.SetVisibility` _children true false))

(event `/Game/Interaction_BP_Root_NULL.Exit Interact`
  (`AkGameplayStatics.SetState` "Book" "Close")
  (`AkComponent.PostAkEvent` (`self.Ak`) "/Game/WwiseSFX/Events/GeneralHouse/Book.Book" "")
  (`LightComponent.SetIntensity` (`self.SpotLight`) 0.0)
  (`SceneComponent.SetVisibility` (`self.OpenBook`) false false)
  (`SceneComponent.SetVisibility` (`self.ClosedBook`) true false)
  (`PlayerController.SetViewTargetWithBlend` (`GameplayStatics.GetPlayerController` 0) (`GameplayStatics.GetPlayerCharacter` 0) 1.0 "VTBlend_Linear" 0.0 true)
  (`SceneComponent.SetVisibility` (`SceneComponent.GetChildrenComponents` (`KismetArrayLibrary.Array_Get` (`|MakeArray` (`self.StaticMesh`) (`self.StaticMesh1`)) (`self.Page`)) false) false false))

(fn `UserConstructionScript`)