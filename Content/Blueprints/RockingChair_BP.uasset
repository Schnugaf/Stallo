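; Rocking chair actor that sets its rotation every tick while an event flag is on, toggled by SpawnEvent and StopEvent.
; Tick accumulates time only while active and applies the rotator returned by DoAwesomeSHit.
; That function holds a sine-driven lerp of roll between Forward and Backward, preserving current pitch and yaw.
; The rotator node appears unconnected to the function's output.
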(event `/Game/Interaction_BP_Root_NULL.StopEvent`
  (set `self.Event` false))

(event `/Game/Interaction_BP_Root_NULL.SpawnEvent`
  (params (EventNr :type Integer))
  (set `self.Event` true))

(event `self.ReceiveTick`
  (params (DeltaSeconds :type "Float (single-precision)"))
  (if (`self.Event`)
    (set `self.Time` (+ DeltaSeconds (`self.Time`)))
    (`self.K2_SetActorRotation` (`self.DoAwesomeSHit`))))

(fn `UserConstructionScript`)