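; Interactable closet Blueprint with two doors that swing open and closed in mirror image.
; Interact toggles the Open state, flips the timer direction and posts a Wwise sound, with ClosetDoorShut on opening and ClosedDoorOpen on closing.
; Tick advances OpenTimer until it passes either end, using its clamped value to lerp door yaw between zero and Rotation, negated for the right door.
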(event `/Game/Interaction_BP_Root_NULL.Interact`
  (bind _ak (`self.Ak`))
  (if (`self.Open`)
    (set `self.Multiplyer` -1.0)
    (set `self.Open` false)
    (`AkComponent.PostAkEvent` _ak "/Game/WwiseSFX/Events/LivingRoom/ClosetDoor/ClosedDoorOpen.ClosedDoorOpen" "")
    (else
      (set `self.Multiplyer` 1.0)
      (set `self.Open` true)
      (`AkComponent.PostAkEvent` _ak "/Game/WwiseSFX/Events/LivingRoom/ClosetDoor/ClosetDoorShut.ClosetDoorShut" ""))))

(event `self.ReceiveTick`
  (params (DeltaSeconds :type "Float (single-precision)"))
  (bind _multiplyer (`self.Multiplyer`))
  (bind _opentimer (`self.OpenTimer`))
  (bind _returnvalue (`KismetMathLibrary.Lerp` 0.0 (`self.Rotation`) (`KismetMathLibrary.FClamp` (`self.OpenTimer`))))
  (if (not (or (and (> _multiplyer 0.5) (>= _opentimer 1.0)) (and (< _multiplyer -0.5) (<= _opentimer 0.0))))
    (bind _output_get (set `self.OpenTimer` (+ (stale _output_get) (* DeltaSeconds (`self.Multiplyer`)))))
    (`SceneComponent.K2_SetRelativeRotation` (`self.LeftDoor`) (`KismetMathLibrary.MakeRotator` 0.0 0.0 _returnvalue) false false)
    (`SceneComponent.K2_SetRelativeRotation` (`self.RightDoor`) (`KismetMathLibrary.MakeRotator` 0.0 0.0 (* _returnvalue -1.0)) false false)))

(fn `UserConstructionScript`)