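; Window actor that, when interacted with, lets light in and can set off a mirror's reflection, likely as part of a light puzzle.
; Interact raises the intensity and bloom scale of its directional light, then line traces forward on the Visibility channel.
; If the first blocking hit is a Mirror_BP_Actor_NULL, it calls that mirror's MirrorReflectonMessage.
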(event `/Game/Blueprint/Interaction_BP_Root_NULL.Interact`
  (bind _returnvalue (`self.K2_GetActorLocation`))
  (bind _directionallight (`self.DirectionalLight`))
  (`LightComponent.SetIntensity` _directionallight 20.0)
  (`LightComponent.SetBloomScale` _directionallight 20.0)
  (bind _outhit (`KismetSystemLibrary.LineTraceSingle` _returnvalue (+ _returnvalue (* (`self.GetActorForwardVector`) 5000.0)) "TraceTypeQuery1"))
  (if (`GameplayStatics.BreakHitResult` _outhit)
    (bind _asmirror_bp_actor_null (cast `/Game/Blueprint/Mirror_BP_Actor_NULL` (`.HitActor` (`GameplayStatics.BreakHitResult` _outhit))))
    (message `/Game/Blueprint/Interaction_BP_Root_NULL.MirrorReflecton` _asmirror_bp_actor_null)))

(fn `UserConstructionScript`)