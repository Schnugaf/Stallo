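; Mirror actor that can be rotated by interaction and fakes a view-dependent reflection with a SceneCaptureComponent2D.
; Each tick, the capture is turned to the mirror's rotation combined with a yaw from the player camera's forward vector, flipped in X and Z.
; Interact adds a small yaw step to the mirror and shows a rotate message.
; MirrorReflecton flags a reflection, sets four point lights' intensity and shows its message.
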(event `/Game/Blueprint/Interaction_BP_Root_NULL.MirrorReflecton`
  (set `self.Has Reflection` true)
  (`LightComponent.SetIntensity` (`self.PointLight`) 5000.0)
  (`LightComponent.SetIntensity` (`self.PointLight2`) 5000.0)
  (`LightComponent.SetIntensity` (`self.PointLight4`) 5000.0)
  (`LightComponent.SetIntensity` (`self.PointLight1`) 5000.0)
  (message `/Game/Blueprint/Interaction_BP_Root_NULL.MirrorReflecton` (`self.Text`)))

(event `/Game/Blueprint/Interaction_BP_Root_NULL.Interact`
  (bind _mirror (`self.Mirror`))
  (`SceneComponent.K2_SetRelativeRotation` _mirror (`KismetMathLibrary.ComposeRotators` (`KismetMathLibrary.MakeRotator` 0.0 0.0 5.0) (`SceneComponent.K2_GetComponentRotation` _mirror)) false false)
  (message `/Game/Blueprint/Interaction_BP_Root_NULL.Rotate` (`self.Text`)))

(event `self.ReceiveTick`
  (params (DeltaSeconds :type "Float (single-precision)"))
  (`SceneComponent.K2_SetWorldRotation` (`self.SceneCaptureComponent2D`) (`KismetMathLibrary.ComposeRotators` (`SceneComponent.K2_GetComponentRotation` (`self.Mirror`)) (`KismetMathLibrary.MakeRotator` 0.0 0.0 (.yaw (`KismetMathLibrary.Conv_VectorToRotator` (* (`KismetMathLibrary.GetForwardVector` (`PlayerCameraManager.GetCameraRotation` (`PlayerController.PlayerCameraManager` (`GameplayStatics.GetPlayerController` 0)))) (-1.0 1.0 -1.0)))))) false false))

(fn `UserConstructionScript`)