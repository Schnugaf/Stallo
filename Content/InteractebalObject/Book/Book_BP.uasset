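; Interactable book actor that the player opens to read pages, with a level-dependent item message for the tutorial versus other levels.
; Interacting swaps closed and open meshes, turns on spotlights, plays a Wwise sound and blends the view to the book's camera.
; ChangeTarget cycles through visible pages, and exiting reverses the setup.
; The book starts with two pages, and SpawnEvent appends further page pairs by event number.
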(event `self.ReceiveBeginPlay`
  (bind _pages (`self.Pages`))
  (`KismetArrayLibrary.Array_Clear` _pages)
  (`KismetArrayLibrary.Array_Add` _pages (`self.Page1`))
  (`KismetArrayLibrary.Array_Add` _pages (`self.Page2`))
  (bind _returnvalue (`GameplayStatics.GetCurrentLevelName` true))
  (if (`KismetStringLibrary.EqualEqual_StrStr` _returnvalue "Tutorial")
    (set `self.ItemMessage` (`self.TotarialMessage`))
    (else
      (set `self.ItemMessage` (`self.GameLvLMessege`)))))

(event `/Game/Interaction_BP_Root_NULL.SpawnEvent`
  (params (EventNr :type Integer))
  (bind _pages (`self.Pages`))
  (switch `int` EventNr
    (:`0`
      (`KismetArrayLibrary.Array_Add` _pages (`self.Page3`))
      (`KismetArrayLibrary.Array_Add` _pages (`self.Page4`)))
    (:`1`
      (`KismetArrayLibrary.Array_Add` _pages (`self.Page5`))
      (`KismetArrayLibrary.Array_Add` _pages (`self.Page6`)))
    (:`2`
      (`KismetArrayLibrary.Array_Add` _pages (`self.Page7`))
      (`KismetArrayLibrary.Array_Add` _pages (`self.Page8`)))))

(event `/Game/Interaction_BP_Root_NULL.Interact`
  (`AkGameplayStatics.SetState` "Book" "Open")
  (`AkComponent.PostAkEvent` (`self.Ak`) "/Game/WwiseSFX/Events/GeneralHouse/Book.Book" "")
  (`LightComponent.SetIntensity` (`self.SpotLight1`) 1000.0)
  (`LightComponent.SetIntensity` (`self.SpotLight`) 1000.0)
  (`SceneComponent.SetVisibility` (`self.OpenBook`) true false)
  (`SceneComponent.SetVisibility` (`self.ClosedBook`) false false)
  (`PlayerController.SetViewTargetWithBlend` (`GameplayStatics.GetPlayerController` 0) (`ActorComponent.GetOwner` (`self.Camera`)) 1.0 "VTBlend_Linear" 0.0 true)
  (`SceneComponent.SetVisibility` (`KismetArrayLibrary.Array_Get` (`self.Pages`) (`self.Page`)) true false))

(event `/Game/Interaction_BP_Root_NULL.ChangeTarget`
  (bind _pages (`self.Pages`))
  (bind _item (`KismetArrayLibrary.Array_Get` _pages (`self.Page`)))
  (`SceneComponent.SetVisibility` _item false false)
  (bind _output_get (set `self.Page` (+ (stale _output_get) 1)))
  (if (> (`self.Page`) (`KismetArrayLibrary.Array_LastIndex` _pages))
    (set `self.Page` 0))
  (`SceneComponent.SetVisibility` _item true false))

(event `/Game/Interaction_BP_Root_NULL.Exit Interact`
  (`AkGameplayStatics.SetState` "Book" "Close")
  (`AkComponent.PostAkEvent` (`self.Ak`) "/Game/WwiseSFX/Events/GeneralHouse/Book.Book" "")
  (`LightComponent.SetIntensity` (`self.SpotLight1`) 0.0)
  (`LightComponent.SetIntensity` (`self.SpotLight`) 0.0)
  (`SceneComponent.SetVisibility` (`self.OpenBook`) false false)
  (`SceneComponent.SetVisibility` (`self.ClosedBook`) true false)
  (`PlayerController.SetViewTargetWithBlend` (`GameplayStatics.GetPlayerController` 0) (`GameplayStatics.GetPlayerCharacter` 0) 1.0 "VTBlend_Linear" 0.0 true)
  (`SceneComponent.SetVisibility` (`KismetArrayLibrary.Array_Get` (`self.Pages`) (`self.Page`)) false false))

(fn `UserConstructionScript`)